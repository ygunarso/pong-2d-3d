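; Physics-driven ball actor, apparently for a 3D menu, that bounces between boundary volumes.
; On BeginPlay it launches its static mesh with a fixed diagonal velocity.
; Overlapping a BP_3D_Boundary negates one velocity component based on the boundary's X or Y tag, defaulting to Z otherwise, instead of relying on collision response.
; Each bounce plays a collision sound at the world origin rather than at the ball.
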(event EventBeginPlay
  (Physics|SetPhysicsLinearVelocity (Variables|Default|GetStaticMesh) "1000.000000,1000.000000,1000.000000" false "None"))

(event Collision|EventActorBeginOverlap
  (params (OtherActor :type Actor%20Object%20Reference))
  (bind _asbp_3d_boundary (Utilities|Casting|CastToBP_3D_Boundary OtherActor))
  (if (Actor|ActorHasTag _asbp_3d_boundary "X")
    (bind _returnvalue (Physics|GetPhysicsLinearVelocity (Variables|Default|GetStaticMesh) "None"))
    (Physics|SetPhysicsLinearVelocity (Variables|Default|GetStaticMesh) (Math|Vector|MakeVector (* (.X (Math|Vector|BreakVector _returnvalue)) -1.0) (.Y (Math|Vector|BreakVector _returnvalue)) (.Z (Math|Vector|BreakVector _returnvalue))) false "None")
    (elif (Actor|ActorHasTag _asbp_3d_boundary "Y")
      (bind _returnvalue_2 (Physics|GetPhysicsLinearVelocity (Variables|Default|GetStaticMesh) "None"))
      (Physics|SetPhysicsLinearVelocity (Variables|Default|GetStaticMesh) (Math|Vector|MakeVector (.X (Math|Vector|BreakVector _returnvalue_2)) (* (.Y (Math|Vector|BreakVector _returnvalue_2)) -1.0) (.Z (Math|Vector|BreakVector _returnvalue_2))) false "None")
      (else
        (bind _returnvalue_3 (Physics|GetPhysicsLinearVelocity (Variables|Default|GetStaticMesh) "None"))
        (Physics|SetPhysicsLinearVelocity (Variables|Default|GetStaticMesh) (Math|Vector|MakeVector (.X (Math|Vector|BreakVector _returnvalue_3)) (.Y (Math|Vector|BreakVector _returnvalue_3)) (* (.Z (Math|Vector|BreakVector _returnvalue_3)) -1.0)) false "None"))))
  (Audio|PlaySoundatLocation "/Game/Audio/S_ballCollision.S_ballCollision" "0, 0, 0" "0, 0, 0" 1.0 1.0 0.0 0 0 0))

(fn ConstructionScript)