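; Ball for a 3D Pong-style match that launches along Y and handles bouncing, scoring and match end.
; Overlaps drive it: paddles reverse Y and set X/Z from paddle velocity plus random spread, while boundaries flip X or Z by "Side" tag.
; Goals recenter and relaunch the ball, updating tagged Text3D scores.
; When either score exceeds six, Tick stops the ball and reloads P1_3D after a delay.
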(event EventBeginPlay
  (Physics|SetPhysicsLinearVelocity (Variables|Default|GetStaticMesh) "0,1000.000000, 0" false "None"))

(event Collision|EventActorBeginOverlap
  (params (OtherActor :type Actor%20Object%20Reference))
  (bind _asbp_3d_paddle_pawn_r (Utilities|Casting|CastToBP_3D_Paddle_Pawn_R OtherActor)
    (:then
      (bind _returnvalue (Physics|GetPhysicsLinearVelocity (Variables|/Game/Blueprints/BP_3D_Paddle_Pawn_R.BP_3D_Paddle_Pawn_R_C|GetPaddle_Mesh _asbp_3d_paddle_pawn_r) "None"))
      (bind _returnvalue_2 (Physics|GetPhysicsLinearVelocity (Variables|Default|GetStaticMesh) "None"))
      (Physics|SetPhysicsLinearVelocity (Variables|Default|GetStaticMesh) (Math|Vector|MakeVector (+ (.X (Math|Vector|BreakVector _returnvalue)) (Math|Random|RandomFloatinRange -1e+03 1e+03)) (* (.Y (Math|Vector|BreakVector _returnvalue_2)) -1.0) (+ (.Z (Math|Vector|BreakVector _returnvalue)) (Math|Random|RandomFloatinRange -1e+03 1e+03))) false "None")
      (Audio|PlaySoundatLocation "/Game/Audio/S_ballCollision.S_ballCollision" "0, 0, 0" "0, 0, 0" 1.0 1.0 0.0 0 0 0))
    (:CastFailed
      (bind _asbp_enemy_paddle_3d (Utilities|Casting|CastToBP_EnemyPaddle_3D OtherActor)
        (:then
          (bind _returnvalue_3 (Physics|GetPhysicsLinearVelocity (Variables|/Game/Blueprints/BP_EnemyPaddle_3D.BP_EnemyPaddle_3D_C|GetStaticMesh _asbp_enemy_paddle_3d) "None"))
          (bind _returnvalue_4 (Physics|GetPhysicsLinearVelocity (Variables|Default|GetStaticMesh) "None"))
          (Physics|SetPhysicsLinearVelocity (Variables|Default|GetStaticMesh) (Math|Vector|MakeVector (+ (.X (Math|Vector|BreakVector _returnvalue_3)) (Math|Random|RandomFloatinRange -1e+03 1e+03)) (* (.Y (Math|Vector|BreakVector _returnvalue_4)) -1.0) (+ (.Z (Math|Vector|BreakVector _returnvalue_3)) (Math|Random|RandomFloatinRange -1e+03 1e+03))) false "None")
          (Audio|PlaySoundatLocation "/Game/Audio/S_ballCollision.S_ballCollision" "0, 0, 0" "0, 0, 0" 1.0 1.0 0.0 0 0 0))
        (:CastFailed
          (bind _asbp_3d_boundary (Utilities|Casting|CastToBP_3D_Boundary OtherActor)
            (:then
              (if (Actor|ActorHasTag _asbp_3d_boundary "Side")
                (bind _returnvalue_5 (Physics|GetPhysicsLinearVelocity (Variables|Default|GetStaticMesh) "None"))
                (Physics|SetPhysicsLinearVelocity (Variables|Default|GetStaticMesh) (Math|Vector|MakeVector (* (.X (Math|Vector|BreakVector _returnvalue_5)) -1.0) (.Y (Math|Vector|BreakVector _returnvalue_5)) (.Z (Math|Vector|BreakVector _returnvalue_5))) false "None")
                (Audio|PlaySoundatLocation "/Game/Audio/S_ballCollision.S_ballCollision" "0, 0, 0" "0, 0, 0" 1.0 1.0 0.0 0 0 0)
                (else
                  (bind _returnvalue_6 (Physics|GetPhysicsLinearVelocity (Variables|Default|GetStaticMesh) "None"))
                  (Physics|SetPhysicsLinearVelocity (Variables|Default|GetStaticMesh) (Math|Vector|MakeVector (.X (Math|Vector|BreakVector _returnvalue_6)) (.Y (Math|Vector|BreakVector _returnvalue_6)) (* (.Z (Math|Vector|BreakVector _returnvalue_6)) -1.0)) false "None")
                  (Audio|PlaySoundatLocation "/Game/Audio/S_ballCollision.S_ballCollision" "0, 0, 0" "0, 0, 0" 1.0 1.0 0.0 0 0 0))))
            (:CastFailed
              (Utilities|Casting|CastToBP_Enemy_Goal_3D OtherActor
                (:then
                  (Transformation|SetActorLocation "0, 0, 0" false false)
                  (Physics|SetPhysicsLinearVelocity (Variables|Default|GetStaticMesh) "0,2000.000000, 0" false "None")
                  (Audio|PlaySoundatLocation "/Game/Audio/S_ballGoal.S_ballGoal" "0, 0, 0" "0, 0, 0" 1.0 1.0 0.0 0 0 0)
                  (Variables|Default|SetP1_Score (+ (Variables|Default|GetP1_Score) 1))
                  (bind _outactors (Actor|GetAllActorsOfClass "/Script/Text3D.Text3DActor"))
                  (for _array_element _outactors
                    (if (Components|ComponentHasTag (Variables|/Script/Engine.Actor|GetRootComponent _array_element) "P1_Score_Tag")
                      (Class|Text3DComponent|SetText (Variables|/Script/Text3D.Text3DActor|GetText3DComponent _array_element) (Utilities|Text|ToText(Integer) (Variables|Default|GetP1_Score)))
                      (if (> (Variables|Default|GetP1_Score) 6)
                        (Variables|Default|SetGameOver true)))))
                (:CastFailed
                  (Utilities|Casting|CastToBP_P1_Goal_3D OtherActor)
                  (Transformation|SetActorLocation "0, 0, 0" false false)
                  (Physics|SetPhysicsLinearVelocity (Variables|Default|GetStaticMesh) "0,-2000.000000, 0" false "None")
                  (Audio|PlaySoundatLocation "/Game/Audio/S_ballGoal.S_ballGoal" "0, 0, 0" "0, 0, 0" 1.0 1.0 0.0 0 0 0)
                  (Variables|Default|SetEnemy_Score (+ (Variables|Default|GetEnemy_Score) 1))
                  (bind _outactors_2 (Actor|GetAllActorsOfClass "/Script/Text3D.Text3DActor"))
                  (for _array_element_2 _outactors_2
                    (if (Components|ComponentHasTag (Variables|/Script/Engine.Actor|GetRootComponent _array_element_2) "Enemy_Score_Tag")
                      (Class|Text3DComponent|SetText (Variables|/Script/Text3D.Text3DActor|GetText3DComponent _array_element_2) (Utilities|Text|ToText(Integer) (Variables|Default|GetEnemy_Score)))
                      (if (> (Variables|Default|GetEnemy_Score) 6)
                        (Variables|Default|SetGameOver true)))))))))))))

(event EventTick
  (params (DeltaSeconds :type Float%20%28single-precision%29))
  (if (Variables|Default|GetGameOver)
    (Physics|SetPhysicsLinearVelocity (Variables|Default|GetStaticMesh) "0, 0, 0" false "None")
    (Utilities|FlowControl|Delay 3.0)
    (bind _outactors (Actor|GetAllActorsOfClass "/Game/Blueprints/BP_Paddle_L.BP_Paddle_L_C"))
    (if (> (Utilities|Array|Length _outactors) 0)
      (Game|OpenLevel(byName) "P1_3D")
      (else
        (Game|OpenLevel(byName) "P1_3D")))))

(fn ConstructionScript)