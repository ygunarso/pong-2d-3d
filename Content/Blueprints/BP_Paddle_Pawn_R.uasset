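; BP_Paddle_Pawn_R is a paddle pawn, apparently the right-hand one, that the player moves along the world X axis.
; Each tick it reads the P1_MoveUp input axis and applies a scaled physics force to PaddleMesh.
; When the actor passes either X limit, it is snapped just back inside the bounds instead, and no force is applied that tick.
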(event EventBeginPlay)

(event Collision|EventActorBeginOverlap
  (params (OtherActor :type Actor%20Object%20Reference)))

(event EventTick
  (params (DeltaSeconds :type Float%20%28single-precision%29))
  (bind _returnvalue (Transformation|GetActorLocation))
  (bind _returnvalue_2 (Transformation|GetActorLocation))
  (bind (_x _y _z) (Math|Vector|BreakVector _returnvalue_2))
  (bind (_x_2 _y_2 _z_2) (Math|Vector|BreakVector _returnvalue))
  (if (> (.X (Math|Vector|BreakVector (Transformation|GetActorLocation))) 1.5e+03)
    (Transformation|SetActorLocation (Math|Vector|MakeVector 1499.0 _y _z) false false)
    (elif (< (.X (Math|Vector|BreakVector (Transformation|GetActorLocation))) -1.5e+03)
      (Transformation|SetActorLocation (Math|Vector|MakeVector -1499.0 _y_2 _z_2) false false)
      (else
        (Physics|AddForce (Variables|Default|GetPaddle_Mesh) (Math|Vector|MakeVector (* (Input|AxisValues|GetP1_MoveUp) 1e+07) 0.0 0.0) "None" false)))))

(fn ConstructionScript)